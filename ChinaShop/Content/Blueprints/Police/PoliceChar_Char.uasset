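; Police enemy character that chases the player and shoots at them once within range.
; Tick moves it toward the player with simple AI navigation, holds position inside a set radius, and destroys it when Health runs out.
; Shoot spawns an explosion effect and a bullet at an arrow component, rate-limited by a DoOnce reset after a delay.
; Overlapping the player costs the police character one Health.
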(event EventBeginPlay)

(event Collision|EventActorBeginOverlap
  (params (OtherActor :type Actor%20Object%20Reference))
  ;[1 1 1] When the player collides with the enemy
  (if (== OtherActor (Game|Player|GetPlayerPawn 0)) ; If true, then the object collided with is a player
    (bind _result (Math|Integer|DecrementInt (Variables|Default|GetHealth))
      (:%20%20
        (Variables|Default|SetHealth _result)))))

(event EventTick
  (params (DeltaSeconds :type Float%20%28single-precision%29))
  (bind _returnvalue (Game|Player|GetPlayerPawn 0))
  (bind _self self)
  (bind _returnvalue_2 (Pawn|GetController _self))
  (Variables|Default|SetThedelta DeltaSeconds)
  (Utilities|FlowControl|Sequence
    (:then_0
      ;[1 1 1] Moving
      (if (< (Transformation|GetDistanceTo _returnvalue) (Variables|Default|GetDistanceAroundPlayer))
        (AI|Navigation|SimpleMovetoLocation _returnvalue_2 (Transformation|GetActorLocation _self))
        (else
          (AI|Navigation|SimpleMovetoActor _returnvalue_2 _returnvalue))))
    (:then_1
      ;[1 1 1] Shooting Mechanic
      (if (< (Transformation|GetDistanceTo (Game|Player|GetPlayerPawn 0)) (Variables|Default|GetDistance%20to%20shoot))
        (Utilities|FlowControl|DoOnce false :!label _label
          (:Completed
            (CallFunction|Shoot)
            (Utilities|FlowControl|Delay (Variables|Default|GetWaitDelay))
            (goto _label Reset)))))
    (:then_2
      ;[1 1 1] Actor Death
      (if (< (Variables|Default|GetHealth) 1)
        (Development|PrintString "Death")
        (Actor|DestroyActor)))))

(fn ConstructionScript)

(fn Shoot
  (bind _arrow1 (Variables|Default|GetArrow1))
  (bind _returnvalue (Transformation|GetWorldTransform _arrow1))
  (bind _returnvalue_2 (Transformation|GetWorldTransform _arrow1))
  (Effects|SpawnEmitteratLocation "/Game/StarterContent/Particles/P_Explosion.P_Explosion" (.location _returnvalue) (.rotation _returnvalue) (.scale _returnvalue))
  (Game|SpawnActorfromClass "/Game/Blueprints/Police/Bullet.Bullet_C" (Math|Transform|MakeTransform (.location _returnvalue_2) (.rotation _returnvalue_2) "0.100000,0.010000,0.100000") "Undefined" 0 0)
  (Development|PrintString "BANG BANG"))