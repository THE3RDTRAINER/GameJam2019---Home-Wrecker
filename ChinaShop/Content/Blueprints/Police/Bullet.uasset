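; Bullet actor for the police enemies that turns to face the player's pawn when play begins.
; Overlap and hit events share one check that the other actor is not its parent PoliceChar_Char, but the branch leads to no action.
; The AddForce and DestroyActor nodes are disconnected, so this graph neither propels nor destroys the bullet.
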(event EventBeginPlay
  (Transformation|SetActorRotation (Math|Rotator|FindLookatRotation (Transformation|GetActorLocation) (Transformation|GetActorLocation (Game|Player|GetPlayerPawn 0)))))

(event Collision|EventActorBeginOverlap
  (params (OtherActor :type Actor%20Object%20Reference))
  (bind _returnvalue (Actor|GetParentActor))
  (bind _aspolice_char_char (Utilities|Casting|CastToPoliceChar_Char _returnvalue))
  (if (or (!= OtherActor _aspolice_char_char) (!= _aspolice_char_char (stale Collision|EventHit Other)))
    _))

(event Collision|EventHit
  (params (MyComp :type Primitive%20Component%20Object%20Reference) (Other :type Actor%20Object%20Reference) (OtherComp :type Primitive%20Component%20Object%20Reference) (bSelfMoved :type Boolean) (HitLocation :type Vector :default "0, 0, 0") (HitNormal :type Vector :default "0, 0, 0") (NormalImpulse :type Vector :default "0, 0, 0") (Hit :type Hit%20Result%20Structure%20%28by%20ref%29))
  (bind _returnvalue (Actor|GetParentActor))
  (bind _aspolice_char_char (Utilities|Casting|CastToPoliceChar_Char _returnvalue))
  (if (or (!= (stale Collision|EventActorBeginOverlap OtherActor) _aspolice_char_char) (!= _aspolice_char_char Other))
    _))

(fn ConstructionScript)