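; Destructible building actor that loses health when the referenced player object hits or overlaps it, then breaks apart and is removed.
; Construction applies the mesh, material, transform and collision box scale, and sets the point value from Health.
; RemoveHealth identifies the player by display-name comparison, decrementing Health with a hit sound.
; Tick watches for depleted Health, then once triggers particles, destructible damage and sound before a delayed destroy.
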(event Collision|EventActorBeginOverlap
  (params (OtherActor :type Actor%20Object%20Reference))
  (Development|PrintString (Utilities|GetDisplayName OtherActor))
  (CallFunction|RemoveHealth OtherActor (Variables|Coding|GetPlayerObjectReference)))

(event EventTick
  (params (DeltaSeconds :type Float%20%28single-precision%29))
  (if (<= (Variables|Design|GetHealth) 0) ; Start Destruction
    (Utilities|FlowControl|DoOnce false
      (:Completed
        (CallFunction|StartDestruction)
        (Development|PrintString (Utilities|String|Append "The Game Object: " (Utilities|GetObjectName self) " is being destroyed!"))
        (Utilities|FlowControl|Delay (Variables|Design|GetTimeToDelay))
        (Actor|DestroyActor)))))

(event Collision|EventHit
  (params (MyComp :type Primitive%20Component%20Object%20Reference) (Other :type Actor%20Object%20Reference) (OtherComp :type Primitive%20Component%20Object%20Reference) (bSelfMoved :type Boolean) (HitLocation :type Vector :default "0, 0, 0") (HitNormal :type Vector :default "0, 0, 0") (NormalImpulse :type Vector :default "0, 0, 0") (Hit :type Hit%20Result%20Structure%20%28by%20ref%29))
  (CallFunction|RemoveHealth Other (Variables|Coding|GetPlayerObjectReference)))

(fn ConstructionScript
  (bind _collisionboxsize (Variables|Default|GetCollisionBoxSize))
  (bind _destructible (Variables|Default|GetDestructible))
  (Variables|Default|SetnumOfPoints (Variables|Design|GetHealth))
  (Class|DestructibleComponent|SetDestructibleMesh _destructible (Variables|Coding|GetDestructibleMesh))
  (Rendering|Material|SetMaterial _destructible 0 (Variables|Default|GetDestructMaterial))
  (Transformation|SetRelativeTransform (Variables|Default|GetDestructible) (Variables|Default|GetDestructTransform) false false)
  (Transformation|SetRelativeScale3D (Variables|Default|GetBoxCollider) (Math|Vector|MakeVector _collisionboxsize _collisionboxsize _collisionboxsize))
  (if (> (Variables|Design|GetHealth) 1)
    _))

(fn StartDestruction
  (bind _self self)
  (bind _returnvalue (Transformation|GetActorLocation _self))
  ;[1 1 1] Emitter for particles, and soon destructables
  (Effects|SpawnEmitteratLocation 0 "0, 0, 0")
  (Class|DestructibleComponent|ApplyDamage (Variables|Default|GetDestructible) 1.0 _returnvalue _returnvalue 0.0)
  (Audio|SpawnSoundatLocation (Variables|Art|GetDestructionSounds) (Transformation|GetActorLocation self) "0, 0, 0" 1.0 1.0 0.0 0 0))

(fn RemoveHealth
  (params (Object :type Object%20Object%20Reference) (PlayerObject :type Object%20Object%20Reference))
  (bind _returnvalue (Utilities|GetDisplayName Object))
  (bind _returnvalue_2 (Utilities|GetDisplayName PlayerObject))
  (if (Utilities|Enum|Equal(Enum) _returnvalue _returnvalue_2)
    (bind _result (Math|Integer|DecrementInt (Variables|Design|GetHealth))
      (:%20%20
        (bind _output_get (Variables|Design|SetHealth _result)) ; Lower Health
        (Development|PrintString (Utilities|String|Append "health is now: " (Utilities|String|ToString(Integer) _output_get)))
        (Audio|SpawnSoundatLocation (Variables|Art|GetHitSound) (Transformation|GetActorLocation self) "0, 0, 0" 1.0 1.0 0.0 0 0)))
    (else
      (Development|PrintString (Utilities|String|Append _returnvalue " is being compared to " _returnvalue_2)))))

(fn UIFunctinos
  (params (ParmIn :type Integer))
  (return 0))