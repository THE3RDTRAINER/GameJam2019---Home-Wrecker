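; Trigger-box spawner that spawns an actor of a configurable class when the player overlaps it.
; It identifies the player by comparing display names, spawns at the Arrow's world location and prints debug messages.
; If DoOnce is set, it destroys itself after spawning.
; The construction script places the Arrow from WhereToSpawn and stretches the Box along X by Length.
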(event EventBeginPlay)

(event Collision|EventActorBeginOverlap
  (params (OtherActor :type Actor%20Object%20Reference))
  (if (Utilities|Enum|Equal(Enum) (Utilities|GetDisplayName OtherActor) (Utilities|GetDisplayName (Variables|Default|GetPlayer)))
    (Development|PrintString (Utilities|String|Append "Spawning: " (Utilities|GetClassDisplayName (Variables|Design|GetclassToSpawn))))
    (Game|SpawnActorfromClass (Variables|Design|GetclassToSpawn) (Math|Transform|MakeTransform (Transformation|GetWorldLocation (Variables|Default|GetArrow)) "0, 0, 0" "1,1,1") "Undefined" 0 0)
    (Development|PrintString "car spawned")
    (if (Variables|Default|GetDoOnce)
      (Actor|DestroyActor))))

(event EventTick
  (params (DeltaSeconds :type Float%20%28single-precision%29)))

(fn ConstructionScript
  (Transformation|SetRelativeTransform (Variables|Default|GetArrow) (Variables|Default|GetwhereToSpawn) false false)
  (Transformation|SetWorldScale3D (Variables|Default|GetBox) (Math|Vector|MakeVector (Variables|Default|GetLength) 1.0 1.0)))